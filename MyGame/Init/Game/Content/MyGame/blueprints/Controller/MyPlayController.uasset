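; RTS-style player controller that edge-scrolls the camera pawn and commands groups of MyCharacter units.
; Left-drag drives the MainUI selection box and fills MyTeam with units inside the XY rectangle between two cursor-traced world points.
; Right-click moves the team, A arms an attack-move for the next left-click, and S stops the team.
; Tick nudges the pawn whenever the cursor nears a viewport edge.
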(event `self.ReceiveBeginPlay`
  (bind _asmypawn (cast `/Game/MyGame/blueprints/Pawns/Mypawn` (`GameplayStatics.GetPlayerPawn` 0)))
  (set `self.MyPawn` _asmypawn)
  (bind _returnvalue (`|CreateWidget` "/Game/MyGame/UI/MainUI.MainUI_C"))
  (bind _output_get (set `self.MainUI` _returnvalue))
  (`UserWidget.AddToViewport` _output_get 0))

(event `self.ReceiveTick`
  (params (DeltaSeconds :type "Float (single-precision)"))
  (`self.CamMove`))

(event `Key|LeftMouseButton`
  (params (Key :type "Key Structure"))
  (:`Pressed`
    (if (`self.SetA`)
      (set `self.CurrentMouseCursor` "Default")
      (`self.TeamAttack`)
      (else
        (set `/Game/MyGame/UI/MainUI.IsDrag?` true (`self.MainUI`))
        (set `self.StartMouse` (`self.GetMousePos`))
        (`/Game/MyGame/UI/MainUI.StartDrag` (`self.MainUI`)))))
  (:`Released`
    (if (`self.SetA`)
      (set `self.SetA` false)
      (else
        (set `/Game/MyGame/UI/MainUI.IsDrag?` false (`self.MainUI`))
        (set `self.EndMouse` (`self.GetMousePos`))
        (`self.GetMyTeam`)))))

(event `Key|RightMouseButton`
  (params (Key :type "Key Structure"))
  (:`Pressed`
    (set `self.CurrentMouseCursor` "Default")
    (set `self.SetA` false)
    (`self.TeamMove`)))

(event `Key|A`
  (params (Key :type "Key Structure"))
  (:`Pressed`
    (set `self.CurrentMouseCursor` "Hand")
    (set `self.SetA` true)))

(event `Key|S`
  (params (Key :type "Key Structure"))
  (:`Pressed`
    (`self.TeamStop`)))

(fn `CamMove`
  (bind (_locationx _locationy) (`self.GetMousePosition`))
  (bind (_sizex _sizey) (`self.GetViewportSize`))
  (bind _returnvalue (/ _locationx (`KismetMathLibrary.Conv_IntToDouble` _sizex)))
  (bind _returnvalue_2 (/ _locationy (`KismetMathLibrary.Conv_IntToDouble` _sizey)))
  (`self.K2_AddActorLocalTransform` (`self.MyPawn`) (`KismetMathLibrary.Conv_VectorToTransform` (+ (+ (`KismetMathLibrary.SelectVector` (0.0 20.0 0.0) (0.0 0.0 0.0) (>= _returnvalue 0.95)) (`KismetMathLibrary.SelectVector` (0.0 -20.0 0.0) (0.0 0.0 0.0) (<= _returnvalue 0.05))) (+ (`KismetMathLibrary.SelectVector` (-20.0 0.0 0.0) (0.0 0.0 0.0) (>= _returnvalue_2 0.95)) (`KismetMathLibrary.SelectVector` (20.0 0.0 0.0) (0.0 0.0 0.0) (<= _returnvalue_2 0.05))))) false false))

(fn `GetMousePos`
  (returns (Location :type "Vector Structure"))
  (return (`.Location` (`GameplayStatics.BreakHitResult` (`self.GetHitResultUnderCursorByChannel` "TraceTypeQuery1")))))

(fn `GetMyTeam`
  (`KismetArrayLibrary.Array_Clear` (`self.MyTeam`))
  (bind _outactors (`GameplayStatics.GetAllActorsOfClass` "/Game/MyGame/blueprints/Pawns/MyCharacter.MyCharacter_C"))
  (for _array_element _outactors
    (if (`self.InMouseBox?` (`self.K2_GetActorLocation` _array_element))
      (`KismetArrayLibrary.Array_Add` (`self.MyTeam`) _array_element)
      (`KismetSystemLibrary.PrintString` (`KismetSystemLibrary.GetDisplayName` _array_element)))))

(fn `InMouseBox?`
  (params (Pos :type "Vector Structure"))
  (returns (In :type Boolean))
  (bind _x (.x Pos))
  (bind _y (.y Pos))
  (bind _x_2 (.x (`self.StartMouse`)))
  (bind _y_2 (.y (`self.StartMouse`)))
  (bind _x_3 (.x (`self.EndMouse`)))
  (bind _y_3 (.y (`self.EndMouse`)))
  (return (and (<= _x (`KismetMathLibrary.FMax` _x_2 _x_3)) (>= _x (`KismetMathLibrary.FMin` _x_2 _x_3)) (<= _y (`KismetMathLibrary.FMax` _y_2 _y_3)) (>= _y (`KismetMathLibrary.FMin` _y_2 _y_3)))))

(fn `TeamAttack`
  (for _array_element (`self.MyTeam`)
    (set `/Game/MyGame/blueprints/Pawns/CharacterBase.IsAttack?` true _array_element)
    (`/Game/MyGame/blueprints/Pawns/CharacterBase.MoveLocation` _array_element (`self.GetMousePos`))))

(fn `TeamMove`
  (for _array_element (`self.MyTeam`)
    (set `/Game/MyGame/blueprints/Pawns/CharacterBase.IsAttack?` false _array_element)
    (`/Game/MyGame/blueprints/Pawns/CharacterBase.MoveLocation` _array_element (`self.GetMousePos`))))

(fn `TeamStop`
  (for _array_element (`self.MyTeam`)
    (set `/Game/MyGame/blueprints/Pawns/CharacterBase.IsAttack?` false _array_element)
    (`/Game/MyGame/blueprints/Pawns/CharacterBase.Stop` _array_element false)))

(fn `UserConstructionScript`)