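; Character Blueprint that picks the nearest robot as its current enemy.
; FindEnemy scans all MyRobot actors, accepts a first candidate only within a fixed range, then keeps any that DisFromEnemy rates as close or closer.
; The result is stored in Enemy, left empty when no robot is in range.
; The event graph holds only disabled default stubs, and nothing here calls FindEnemy.
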(fn `FindEnemy`
  (locals (Chosest :type "/Game/MyGame/blueprints/Pawns/CharacterBase Object Reference"))
  (set `local.Chosest` null)
  (bind _outactors (`GameplayStatics.GetAllActorsOfClass` "/Game/MyGame/blueprints/Pawns/MyRobot.MyRobot_C"))
  (for _array_element _outactors
    (if (`KismetSystemLibrary.IsValid` (`local.Chosest`))
      (if (<= (`self.DisFromEnemy` _array_element) (`self.DisFromEnemy` (`local.Chosest`)))
        (set `local.Chosest` _array_element :!label _label))
      (elif (<= (`self.DisFromEnemy` _array_element) 1500.0)
        (goto _label))))
  (set `self.Enemy` (`local.Chosest`))
  (return))

(fn `UserConstructionScript`
  (`parent.UserConstructionScript`))