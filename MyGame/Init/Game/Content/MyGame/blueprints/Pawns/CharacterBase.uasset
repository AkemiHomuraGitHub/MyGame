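; Base character pawn with health, a life bar widget and automatic ranged attacks on an enemy actor.
; While attacking, Tick calls the stub FindEnemy, then moves toward the enemy or, within range, stops and plays a montage whose notify spawns a bullet targeting it.
; A DoOnce with delayed reset throttles shots.
; Damage reduces health; near zero, the same Attack0 montage section plays and its notify destroys the actor.
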(event `self.ReceiveBeginPlay`
  (`self.InitLifeBar`)
  (bind _asmy_play_controller (cast `/Game/MyGame/blueprints/Controller/MyPlayController` (`GameplayStatics.GetPlayerController` 0)))
  (set `self.MyController` _asmy_play_controller))

(event `self.ReceiveTick`
  (params (DeltaSeconds :type "Float (single-precision)"))
  (`self.AttackEvent`))

(event `AttackEvent`
  (if (`self.IsAttack?`)
    (`self.FindEnemy`)
    (if (`KismetSystemLibrary.IsValid` (`self.Enemy`))
      (if (<= (`self.DisFromEnemy` (`self.Enemy`)) (`self.DisAttack`))
        (`self.Stop` true)
        (`/Engine/EditorBlueprintResources/StandardMacros.DoOnce` false :!label _label
          (:`Completed`
            (`self.K2_SetActorRotation` (`self.GetRotation` (`self.Enemy`)))
            (`|PlayMontage` (`self.Mesh`) "/Game/MyGame/animation/MCMontage.MCMontage" 1.0 0.0 "Attack0"
              (:`then`
                (`KismetSystemLibrary.Delay` 1.0)
                (goto _label :!via `Reset`))
              (:`OnNotifyBegin`
                (`self.SpawnBullet`)))))
        (else
          (`self.MoveToEnemy` (`self.Enemy`)))))))

(event `SpawnBullet`
  (bind _returnvalue (`|SpawnActorFromClass` "/Game/MyGame/blueprints/Weapon/MyBullet.MyBullet_C" (`self.GetTransfrom` (`self.Enemy`)) "Undefined" "OverrideRootScale" null null))
  (set `/Game/MyGame/blueprints/Weapon/MyBullet.Enemy` (`self.Enemy`) _returnvalue))

(event `self.ReceiveAnyDamage`
  (params (Damage :type "Float (single-precision)") (DamageType :type "DamageType Object Reference") (InstigatedBy :type "Controller Object Reference") (DamageCauser :type "Actor Object Reference"))
  (bind _dead_ (`self.CheakDead?`))
  (`self.GetDamage` Damage)
  (`KismetSystemLibrary.PrintString` (`KismetStringLibrary.Conv_BoolToString` _dead_))
  (if _dead_
    (`/Engine/EditorBlueprintResources/StandardMacros.DoOnce` false
      (:`Completed`
        (`self.DeadEvent`)))))

(event `DeadEvent`
  (`|PlayMontage` (`self.Mesh`) "/Game/MyGame/animation/MCMontage.MCMontage" 1.0 0.0 "Attack0"
    (:`OnNotifyBegin`
      (`self.K2_DestroyActor`))))

(fn `CheakDead?`
  (returns (`Dead?` :type Boolean))
  (return (<= (`self.Health`) 1.0)))

(fn `DisFromEnemy`
  (params (Enemy :type "/Game/MyGame/blueprints/Pawns/CharacterBase Object Reference"))
  (returns (Distance :type "Float (double-precision)"))
  (if (`KismetSystemLibrary.IsValid` Enemy)
    (return (`KismetMathLibrary.VSize` (- (`self.K2_GetActorLocation` self) (`self.K2_GetActorLocation` Enemy))))
    (else
      (return 10000.0))))

(fn `FindEnemy`
  (return))

(fn `GetDamage`
  (params (Damage :type "Float (double-precision)"))
  (set `self.Health` (`KismetMathLibrary.FMax` (- (`self.Health`) Damage)))
  (return))

(fn `GetRotation`
  (params (Enemy :type "/Game/MyGame/blueprints/Pawns/CharacterBase Object Reference"))
  (returns (Rotation :type "Rotator Structure"))
  (if (`KismetSystemLibrary.IsValid` Enemy)
    (return (`KismetMathLibrary.FindLookAtRotation` (`self.K2_GetActorLocation`) (`self.K2_GetActorLocation` Enemy)))
    (else
      (return (`self.K2_GetActorRotation` self)))))

(fn `GetTransfrom`
  (params (Enemy :type "/Game/MyGame/blueprints/Pawns/CharacterBase Object Reference"))
  (returns (Transform :type "Transform Structure"))
  (return (`KismetMathLibrary.MakeTransform` (`self.K2_GetActorLocation` self) (`self.GetRotation` Enemy))))

(fn `InitLifeBar`
  (bind _asmcstate (cast `/Game/MyGame/UI/MCState` (`WidgetComponent.GetUserWidgetObject` (`self.LifeBar`))))
  (set `/Game/MyGame/UI/MCState.Character` self _asmcstate))

(fn `MoveLocation`
  (params (Pos :type "Vector Structure"))
  (`self.Stop` false)
  (`AIBlueprintHelperLibrary.SimpleMoveToLocation` (`self.GetController` self) Pos))

(fn `MoveToEnemy`
  (params (Enemy :type "/Game/MyGame/blueprints/Pawns/CharacterBase Object Reference"))
  (`AIBlueprintHelperLibrary.SimpleMoveToActor` (`self.GetController` self) Enemy))

(fn `Stop`
  (params (PlayMontage :type Boolean))
  (if (not PlayMontage)
    (`self.StopAnimMontage` "/Game/MyGame/animation/MCMontage.MCMontage"))
  (`MovementComponent.StopMovementImmediately` (`self.CharacterMovement`)))

(fn `UserConstructionScript`)