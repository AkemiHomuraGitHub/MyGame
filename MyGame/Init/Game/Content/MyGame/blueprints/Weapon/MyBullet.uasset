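; MyBullet is a homing projectile actor that chases an assigned Enemy and damages it on contact.
; Each tick it re-aims ProjectileMovement velocity toward the Enemy's location at the initial speed.
; Overlapping that Enemy spawns an explosion particle, applies Damage and destroys the bullet; other overlaps are ignored.
; If the Enemy becomes invalid, the bullet explodes and destroys itself without dealing damage.
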(event `self.ReceiveActorBeginOverlap`
  (params (OtherActor :type "Actor Object Reference"))
  (if (== OtherActor (`self.Enemy`))
    (`GameplayStatics.SpawnEmitterAtLocation` "/Game/StarterContent/Particles/P_Explosion.P_Explosion" (`SceneComponent.K2_GetComponentLocation` (`self.Sphere`)))
    (`self.CauseDamage`)
    (`self.K2_DestroyActor`)))

(event `self.ReceiveTick`
  (params (DeltaSeconds :type "Float (single-precision)"))
  (if (`KismetSystemLibrary.IsValid` (`self.Enemy`))
    (set `MovementComponent.Velocity` (`self.GetNewVelocity` (`self.Enemy`)) (`self.ProjectileMovement`))
    (else
      (`GameplayStatics.SpawnEmitterAtLocation` "/Game/StarterContent/Particles/P_Explosion.P_Explosion" (`SceneComponent.K2_GetComponentLocation` (`self.Sphere`)))
      (`self.K2_DestroyActor`))))

(fn `CauseDamage`
  (`GameplayStatics.ApplyDamage` (`self.Enemy`) (`self.Damage`)))

(fn `GetNewVelocity`
  (params (Enemy :type "/Game/MyGame/blueprints/Pawns/CharacterBase Object Reference"))
  (returns (Velocity :type "Vector Structure"))
  (return (* (`KismetMathLibrary.GetForwardVector` (`KismetMathLibrary.FindLookAtRotation` (`SceneComponent.K2_GetComponentLocation` (`self.Sphere`)) (`self.K2_GetActorLocation` Enemy))) (`ProjectileMovementComponent.InitialSpeed` (`self.ProjectileMovement`)))))

(fn `UserConstructionScript`)